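; Archer tower pawn for a tower defense that turns toward enemies and shoots bullets at them.
; PawnSensing locks the first seen EnemyPawn as target until it stops overlapping TowerRadius.
; While targeted, Tick rotates the tower and calls Shoot, relying on a FireRate Delay to pace staggered volleys of BulletAmount bullets.
; Each bullet receives damage, pierce and one elemental stat: ice slow, fire burn or electric extra damage.
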(event `Shoot`
  ;[1 1 1] Shoot
  (`KismetSystemLibrary.Delay` (`self.Fire Rate`))
  (if (`self.HasTarget`)
    (`SkeletalMeshComponent.PlayAnimation` (`self.Archer`) "/Game/Meshes/Tower/Standing_Aim_Recoil_Anim_mixamo_com.Standing_Aim_Recoil_Anim_mixamo_com" false)
    (`/Engine/EditorBlueprintResources/StandardMacros.ForLoopWithDelay` 1 (`self.BulletAmount`) :!label _label
      (:`LoopBody`
        (bind _returnvalue (`|SpawnActorFromClass` "/Game/Blueprints/Player/Bullet.Bullet_C" (`SceneComponent.K2_GetComponentToWorld` (`self.BulletSpawner`)) "AdjustIfPossibleButAlwaysSpawn" "MultiplyWithRoot" null null))
        (set `self.SpawnedBullet` _returnvalue)
        (`self.Set Bullet Stats`))
      (:`ToDelay`
        (`KismetSystemLibrary.Delay` 0.01)
        (goto _label :!via `FromDelay`)))))

(event `Set Rotation`
  ;[1 1 1] Set Rotation
  (`self.K2_SetActorRotation` (`KismetMathLibrary.RInterpTo_Constant` (`self.K2_GetActorRotation`) (`KismetMathLibrary.Conv_VectorToRotator` (`KismetMathLibrary.GreaterGreater_VectorRotator` (0.0 -90.0 0.0) (`KismetMathLibrary.FindLookAtRotation` (`self.K2_GetActorLocation`) (`self.K2_GetActorLocation` (`self.Current Target`))))) 1.0 10.0)))

(event `Set Bullet Stats`
  (bind _spawnedbullet (`self.SpawnedBullet`))
  ;[1 1 1] Set stats for the bullet
  (if (`KismetSystemLibrary.IsValid` _spawnedbullet)
    (set `/Game/Blueprints/Player/Bullet.BulletDmg` (`self.TowerDmg`) _spawnedbullet)
    (set `/Game/Blueprints/Player/Bullet.Pierce` (`self.PierceAmount`) _spawnedbullet)
    ;[1 1 1] Set Element
    ;;[1 1 1] Ice
    (if (`self.IsIce`)
      (set `/Game/Blueprints/Player/Bullet.SlowAmount` (`self.SlowAmount`) (`self.SpawnedBullet`))
      (else
        ;;[1 1 1] Fire
        (if (`self.IsFire`)
          (set `/Game/Blueprints/Player/Bullet.BurnAmount` (`self.BurnAmount`) (`self.SpawnedBullet`))
          (else
            ;;[1 1 1] Fire
            (if (`self.IsEletric`)
              (set `/Game/Blueprints/Player/Bullet.ExtraDmg` (`self.ExtraDmg`) (`self.SpawnedBullet`)))))))))

(event `self.ReceiveTick`
  (params (DeltaSeconds :type "Float (single-precision)"))
  (if (`self.HasTarget`)
    (if (`PrimitiveComponent.IsOverlappingActor` (`self.TowerRadius`) (`self.Current Target`))
      (`self.Set Rotation`)
      (`self.Shoot`)
      (else
        (set `self.Current Target` null)
        (set `self.HasTarget` false)))))

(event `self.PawnSensing.OnSeePawn`
  (params (Pawn :type "Pawn Object Reference"))
  ;[1 1 1] Get Target
  (if (not (`self.HasTarget`))
    (bind _asenemy_pawn (cast `/Game/Blueprints/Enemy/EnemyPawn` Pawn))
    (set `self.Current Target` _asenemy_pawn)
    (set `self.HasTarget` true)))

(fn `UserConstructionScript`)