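; CustomTower is a tower actor that fires homing bullets at CustomEnemy actors in range.
; Tick selects overlapping enemies whose TimeInSpline exceeds the stored maximum, then rotates and calls Shoot; end overlap resets tracking when the target leaves.
; Shoot waits FireRate, then spawns a short-staggered burst through a delayed loop.
; Each bullet receives damage, pierce, the homing target and one element (ice slow, fire burn or electric extra damage) with matching material.
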(event `Shoot`
  ;[1 1 1] Shoot
  (`KismetSystemLibrary.Delay` (`self.Fire Rate`))
  (`/Engine/EditorBlueprintResources/StandardMacros.ForLoopWithDelay` 1 (`self.BulletAmount`) :!label _label
    (:`LoopBody`
      (bind _returnvalue (`|SpawnActorFromClass` "/Game/Blueprints/Player/Bullet.Bullet_C" (`SceneComponent.K2_GetComponentToWorld` (`self.BulletSpawner`)) "AdjustIfPossibleButAlwaysSpawn" "MultiplyWithRoot" null null))
      (set `self.SpawnedBullet` _returnvalue)
      (`self.Set Bullet Stats`))
    (:`ToDelay`
      (`KismetSystemLibrary.Delay` 0.01)
      (goto _label :!via `FromDelay`))))

(event `Set Rotation`
  ;[1 1 1] Set Rotation
  (`self.K2_SetActorRotation` (`KismetMathLibrary.Conv_VectorToRotator` (`KismetMathLibrary.GreaterGreater_VectorRotator` (0.0 -90.0 0.0) (`KismetMathLibrary.FindLookAtRotation` (`self.K2_GetActorLocation`) (`self.K2_GetActorLocation` (`self.Current Target`)))))))

(event `Set Bullet Stats`
  (bind _spawnedbullet (`self.SpawnedBullet`))
  (bind _spawnedbullet_2 (`self.SpawnedBullet`))
  (bind _spawnedbullet_3 (`self.SpawnedBullet`))
  (bind _spawnedbullet_4 (`self.SpawnedBullet`))
  ;[1 1 1] Set stats for the bullet
  (if (`KismetSystemLibrary.IsValid` _spawnedbullet_3)
    (set `/Game/Blueprints/Player/Bullet.BulletDmg` (`self.TowerDmg`) _spawnedbullet_3)
    (set `/Game/Blueprints/Player/Bullet.Pierce` (`self.PierceAmount`) _spawnedbullet_3)
    (if (`KismetSystemLibrary.IsValid` (`self.Current Target`))
      (set `ProjectileMovementComponent.HomingTargetComponent` (`self.GetComponentByClass` (`self.Current Target`) "/Script/Engine.SceneComponent") (`/Game/Blueprints/Player/Bullet.ProjectileMovement` _spawnedbullet_3))
      ;[1 1 1] Set Element
      ;;[1 1 1] Ice
      (if (`self.IsIce`)
        (set `/Game/Blueprints/Player/Bullet.SlowAmount` (`self.SlowAmount`) _spawnedbullet)
        (`PrimitiveComponent.SetMaterial` (`/Game/Blueprints/Player/Bullet.Bullet` _spawnedbullet) 0 "/Engine/EditorMaterials/WidgetMaterial_Z.WidgetMaterial_Z")
        (else
          ;;[1 1 1] Fire
          (if (`self.IsFire`)
            (set `/Game/Blueprints/Player/Bullet.BurnAmount` (`self.BurnAmount`) _spawnedbullet_2)
            (`PrimitiveComponent.SetMaterial` (`/Game/Blueprints/Player/Bullet.Bullet` _spawnedbullet_2) 0 "/Engine/EditorMaterials/WidgetMaterial_X.WidgetMaterial_X")
            (else
              ;;[1 1 1] Fire
              (if (`self.IsEletric`)
                (set `/Game/Blueprints/Player/Bullet.ExtraDmg` (`self.ExtraDmg`) _spawnedbullet_4)
                (`PrimitiveComponent.SetMaterial` (`/Game/Blueprints/Player/Bullet.Bullet` _spawnedbullet_4) 0 "/Engine/EditorMaterials/WidgetMaterial_Current.WidgetMaterial_Current")))))))))

(event `self.ReceiveTick`
  (params (DeltaSeconds :type "Float (single-precision)"))
  ;[1 1 1] Get Target
  (for _array_element (`PrimitiveComponent.GetOverlappingActors` (`self.TowerColl`) "/Game/Blueprints/Enemy/CustomEnemy.CustomEnemy_C")
    (bind _ascustom_enemy (cast `/Game/Blueprints/Enemy/CustomEnemy` _array_element))
    (bind _timeinspline (`/Game/Blueprints/Enemy/CustomEnemy.TimeInSpline` _ascustom_enemy))
    (if (> _timeinspline (`self.EnemyLowestDistance`))
      (set `self.EnemyLowestDistance` _timeinspline)
      (set `self.Current Target` _ascustom_enemy)
      (`self.Set Rotation`)
      (`self.Shoot`))))

(event `self.ReceiveActorEndOverlap`
  (params (OtherActor :type "Actor Object Reference"))
  ;[1 1 1] Get Target
  (if (`KismetArrayLibrary.Array_IsValidIndex` (`PrimitiveComponent.GetOverlappingActors` (`self.TowerColl`) "/Game/Blueprints/Enemy/CustomEnemy.CustomEnemy_C"))
    (if (not (`PrimitiveComponent.IsOverlappingActor` (`self.TowerColl`) (`self.Current Target`)))
      (set `self.EnemyLowestDistance` 0.0 :!label _label_2)
      (set `self.Current Target` null))
    (else
      (goto _label_2))))

(fn `UserConstructionScript`)