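; GameManager runs a wave-defense match: it creates menu and player UI, loads sound settings, and decides victory or defeat.
; BeginPlay shows the menu in MainMenu, otherwise fills the HUD with player HP.
; Outside MainMenu, Tick updates a real-time clock and wave number from the EnemySpawner, re-adds the HUD to the viewport, and checks the round.
; Zero HP pauses into the defeat panel; finishing wave 40 shows victory.
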(event `CountTime`
  ;[1 1 1] Timer
  (bind _output_get (set `self.Sec` (`KismetMathLibrary.FTrunc` (mod (`GameplayStatics.GetRealTimeSeconds`) 60.0))))
  (set `TextBlock.Text` (`KismetTextLibrary.Conv_IntToText` _output_get) (`/Game/Blueprints/UI/PlayerUI.TimeSec` (`self.PlayerUI_Var`)))
  (bind _output_get_2 (set `self.Min` (`KismetMathLibrary.Conv_Int64ToInt` (`KismetMathLibrary.FFloor64` (/ (`GameplayStatics.GetRealTimeSeconds`) 60.0)))))
  (set `TextBlock.Text` (`KismetTextLibrary.Conv_IntToText` _output_get_2) (`/Game/Blueprints/UI/PlayerUI.TimeMin` (`self.PlayerUI_Var`))))

(event `self.ReceiveBeginPlay`
  ;[1 1 1] Update UI Text
  (`self.LoadSettings`)
  (bind _returnvalue (`GameplayStatics.CreateSaveGameObject` "/Game/Blueprints/Game/MySave.MySave_C"))
  (set `self.SavedGame` _returnvalue)
  (bind _returnvalue_2 (`|CreateWidget` "/Game/Blueprints/UI/MenuUI.MenuUI_C"))
  (bind _returnvalue_3 (`|CreateWidget` "/Game/Blueprints/UI/PlayerUI.PlayerUI_C"))
  (bind _returnvalue_4 (`GameplayStatics.GetCurrentLevelName` true))
  (set `self.MenuUI_Var` _returnvalue_2)
  (if (`KismetStringLibrary.NotEqual_StrStr` _returnvalue_4 "MainMenu")
    (bind _output_get (set `self.PlayerUI_Var` _returnvalue_3))
    (set `TextBlock.Text` (`KismetTextLibrary.Conv_IntToText` (`self.PlayerHP`)) (`/Game/Blueprints/UI/PlayerUI.PlayerHP_Text` _output_get))
    (else
      (`UserWidget.AddToViewport` (`self.MenuUI_Var`) 0))))

(event `self.ReceiveTick`
  (params (DeltaSeconds :type "Float (single-precision)"))
  ;[1 1 1] Update UI Text
  (bind _returnvalue (`GameplayStatics.GetCurrentLevelName` true))
  (if (`KismetStringLibrary.NotEqual_StrStr` _returnvalue "MainMenu")
    (`self.CountTime`)
    (`self.CheckRound`)
    (bind _returnvalue_2 (`GameplayStatics.GetActorOfClass` "/Game/Blueprints/Enemy/EnemySpawner.EnemySpawner_C"))
    (set `TextBlock.Text` (`KismetTextLibrary.Conv_IntToText` (`/Game/Blueprints/Enemy/EnemySpawner.CurrentWave` _returnvalue_2)) (`/Game/Blueprints/UI/PlayerUI.WaveNr_Text` (stale `self.ReceiveBeginPlay` _output_get)))
    (`UserWidget.AddToViewport` (stale `self.ReceiveBeginPlay` _output_get) 0)))

(event `LoadSettings`
  ;[1 1 1] Load Settings
  (bind _asmy_game_instance (cast `/Game/Blueprints/Game/MyGameInstance` (`GameplayStatics.GetGameInstance`)))
  (`/Game/Blueprints/Game/MyGameInstance.LoadSoundSettings` _asmy_game_instance))

(event `CheckRound`
  ;[1 1 1] Check for Victory
  (if (`self.IsOpen`)
    _
    (elif (<= (`self.PlayerHP`) 0)
      (`self.Defeat`)
      (else
        (bind _returnvalue (`GameplayStatics.GetActorOfClass` "/Game/Blueprints/Enemy/EnemySpawner.EnemySpawner_C"))
        (if (`/Game/Blueprints/Enemy/EnemySpawner.HasFinishedWave` _returnvalue)
          (if (== (`/Game/Blueprints/Enemy/EnemySpawner.CurrentWave` _returnvalue) 40)
            (`Widget.SetVisibility` (`/Game/Blueprints/UI/PlayerUI.VictoryPanel` (`self.PlayerUI_Var`)) "Visible")
            (`Widget.SetVisibility` (`/Game/Blueprints/UI/PlayerUI.Upgrades` (`self.PlayerUI_Var`)) "Hidden")
            (`Widget.SetVisibility` (`/Game/Blueprints/UI/PlayerUI.Upgrades_Enemy` (`self.PlayerUI_Var`)) "Hidden")
            (`Widget.SetIsEnabled` (`/Game/Blueprints/UI/PlayerUI.PauseBtn` (`self.PlayerUI_Var`)) false)
            (set `self.IsOpen` true)))))))

(event `Defeat`
  ;[1 1 1] Defeat
  (`GameplayStatics.SetGamePaused` true)
  (set `Widget.bIsEnabled` false (`/Game/Blueprints/UI/PlayerUI.PauseBtn` (`self.PlayerUI_Var`)))
  (`Widget.SetVisibility` (`/Game/Blueprints/UI/PlayerUI.DefeatPanel` (`self.PlayerUI_Var`)) "Visible")
  (`Widget.SetVisibility` (`/Game/Blueprints/UI/PlayerUI.Upgrades` (`self.PlayerUI_Var`)) "Hidden")
  (`Widget.SetVisibility` (`/Game/Blueprints/UI/PlayerUI.Upgrades_Enemy` (`self.PlayerUI_Var`)) "Hidden")
  (set `Widget.bIsEnabled` false (`/Game/Blueprints/UI/PlayerUI.PauseBtn` (`self.PlayerUI_Var`))))

(fn `UserConstructionScript`)