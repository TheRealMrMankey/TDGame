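; MyGameInstance is the game instance that holds music and SFX volume settings and persists them in the Save1 slot.
; LoadSoundSettings reads the slot as a MySave and copies both volumes into its own variables, doing nothing more if the cast fails.
; SaveSoundSettings writes both volumes into the SavedGame object held by the GameManager actor, then saves that object back to the slot.
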(event `LoadSoundSettings`
  (bind _returnvalue (`GameplayStatics.LoadGameFromSlot` "Save1"))
  (bind _asmy_save (cast `/Game/Blueprints/Game/MySave` _returnvalue))
  (set `self.MusicVolume` (`/Game/Blueprints/Game/MySave.MusicVolume` _asmy_save))
  (set `self.SFXVolume` (`/Game/Blueprints/Game/MySave.SFXVolume` _asmy_save)))

(event `SaveSoundSettings`
  (bind _returnvalue (`GameplayStatics.GetActorOfClass` "/Game/Blueprints/Game/GameManager.GameManager_C"))
  (bind _savedgame (`/Game/Blueprints/Game/GameManager.SavedGame` _returnvalue))
  (set `/Game/Blueprints/Game/MySave.MusicVolume` (`self.MusicVolume`) _savedgame)
  (set `/Game/Blueprints/Game/MySave.SFXVolume` (`self.SFXVolume`) _savedgame)
  (`GameplayStatics.SaveGameToSlot` _savedgame "Save1"))