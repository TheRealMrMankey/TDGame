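; Enemy spawner that runs a fixed number of timed waves from BeginPlay, spawning enemy pawns at its Plane's transform.
; Nested delayed loop macros pace waves and individual spawns, with the wave delay running alongside spawning rather than after it.
; Each wave after the first adds the initial per-wave count to its size.
; Random rolls flag each new pawn as armored, elemental-immune, both or neither.
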(event `self.ReceiveBeginPlay`
  (set `self.IncreaseBaseValue` (`self.EnemiesPerWave`))
  (bind _index (`/Engine/EditorBlueprintResources/StandardMacros.ForLoopWithDelay` 1 (`self.NrWaves`) :!label _label)
    (:`LoopBody`
      ;[1 1 1] Set Wave and Enemies per Wave
      (bind _output_get (set `self.CurrentWave` _index))
      (if (not (== _output_get 1))
        (set `self.EnemiesPerWave` (+ (`self.EnemiesPerWave`) (`self.IncreaseBaseValue`))))
      (`self.SpawnEnemies`))
    (:`ToDelay`
      (`KismetSystemLibrary.Delay` (`self.TimeBetweenWaves`))
      (goto _label :!via `FromDelay`))))

(event `SpawnEnemies`
  ;[1 1 1] Spawn Enemies
  (`/Engine/EditorBlueprintResources/StandardMacros.ForLoopWithDelay` 1 (`self.EnemiesPerWave`) :!label _label_2
    (:`LoopBody`
      (bind _returnvalue (`|SpawnActorFromClass` "/Game/Blueprints/Enemy/EnemyPawn.EnemyPawn_C" (`SceneComponent.K2_GetComponentToWorld` (`self.Plane`)) "AlwaysSpawn" "MultiplyWithRoot" null null))
      (set `self.EnemyPawn` _returnvalue)
      (`self.Decide if Armored`)
      (`self.Decide if Ele Immune`))
    (:`ToDelay`
      (`KismetSystemLibrary.Delay` (`self.EnemySpawnRate`))
      (goto _label_2 :!via `FromDelay`))))

(event `Decide if Armored`
  ;[1 1 1] Decide if the spawned Enemy is Armored type
  (if (> (`KismetMathLibrary.RandomInteger` (`self.MaxRandomArmored`)) 0)
    (set `/Game/Blueprints/Enemy/EnemyPawn.IsArmored` true (`self.EnemyPawn`))
    (else
      (set `/Game/Blueprints/Enemy/EnemyPawn.IsArmored` false (`self.EnemyPawn`)))))

(event `Decide if Ele Immune`
  ;[1 1 1] Decide if the spawned Enemy is Armored type
  (if (> (`KismetMathLibrary.RandomInteger` (`self.MaxRandomImmune`)) 0)
    (set `/Game/Blueprints/Enemy/EnemyPawn.ElementalImmune` true (`self.EnemyPawn`))
    (else
      (set `/Game/Blueprints/Enemy/EnemyPawn.ElementalImmune` false (`self.EnemyPawn`)))))

(fn `UserConstructionScript`)