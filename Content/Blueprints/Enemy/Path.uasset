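; Path actor in the Enemy folder that draws a lit track along an editable spline.
; The construction script splits the spline by SectionLenght and adds a spline mesh component per section, with black body and blue light materials.
; Each section takes local positions and tangents from the spline, clamping tangent length to the section length so segments bend cleanly.
; It has no runtime logic.
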(fn `UserConstructionScript`
  (bind _spline (`self.Spline`))
  (bind _sectionlenght (`self.SectionLenght`))
  (bind _sectionlenght_2 (`self.SectionLenght`))
  (for _index (range (+ (`KismetMathLibrary.FTrunc` (/ (`SplineComponent.GetSplineLength` (`self.Spline`)) _sectionlenght)) 1))
    (bind _returnvalue (`AddComponent|NODE_AddSplineMeshComponent-0`))
    (`PrimitiveComponent.SetMaterial` _returnvalue 0 "/Game/Materials/GlobalBlackM.GlobalBlackM")
    (`PrimitiveComponent.SetMaterial` _returnvalue 1 "/Game/Materials/PathLightM_Blue.PathLightM_Blue")
    (`PrimitiveComponent.SetMaterial` _returnvalue 2 "/Game/Materials/PathLightM_Blue.PathLightM_Blue")
    (bind _returnvalue_2 (* _index _sectionlenght))
    (bind _returnvalue_3 (* (+ _index 1) _sectionlenght))
    (`SplineMeshComponent.SetStartAndEnd` _returnvalue (`SplineComponent.GetLocationAtDistanceAlongSpline` _spline _returnvalue_2 "Local") (`KismetMathLibrary.ClampVectorSize` (`SplineComponent.GetTangentAtDistanceAlongSpline` _spline _returnvalue_2 "Local") 0.0 _sectionlenght_2) (`SplineComponent.GetLocationAtDistanceAlongSpline` _spline _returnvalue_3 "Local") (`KismetMathLibrary.ClampVectorSize` (`SplineComponent.GetTangentAtDistanceAlongSpline` _spline _returnvalue_3 "Local") 0.0 _sectionlenght_2) true)))