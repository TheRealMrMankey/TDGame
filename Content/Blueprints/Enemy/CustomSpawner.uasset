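; CustomSpawner is an actor that keeps spawning CustomEnemy actors at its Plane component's transform, ignoring collisions.
; On BeginPlay it doubles global time dilation and starts a near-endless delayed loop, spawning one enemy per iteration.
; Tick re-rolls a random integer from zero to nine every frame, which supplies the dilated delay in seconds between spawns.
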(event `self.ReceiveBeginPlay`
  (`GameplayStatics.SetGlobalTimeDilation` 2.0)
  (`/Engine/EditorBlueprintResources/StandardMacros.ForLoopWithDelay` 1 99999 :!label _label
    (:`LoopBody`
      (`|SpawnActorFromClass` "/Game/Blueprints/Enemy/CustomEnemy.CustomEnemy_C" (`SceneComponent.K2_GetComponentToWorld` (`self.Plane`)) "AlwaysSpawn" "MultiplyWithRoot" null null))
    (:`ToDelay`
      (`KismetSystemLibrary.Delay` (`KismetMathLibrary.Conv_IntToDouble` (`self.Random Time`)))
      (goto _label :!via `FromDelay`))))

(event `self.ReceiveTick`
  (params (DeltaSeconds :type "Float (single-precision)"))
  (set `self.Random Time` (`KismetMathLibrary.RandomInteger` 10)))

(fn `UserConstructionScript`)