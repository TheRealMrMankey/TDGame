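; Enemy pawn that follows the level's Path spline and can be burned or slowed, such as by turret ice shots.
; BeginPlay starts a timeline that moves and rotates it along the spline at a rate derived from TimeToComplete.
; Tick triggers delayed burn damage, reapplies the play rate while slowed, and destroys it at zero life, also checked on timeline updates.
; Armor and elemental immunity checks are empty branches.
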(event `Burn`
  ;[1 1 1] Take damage from burning
  (`KismetSystemLibrary.Delay` 0.5)
  (set `self.EnemyLife` (- (`self.EnemyLife`) (`self.BurnAmount`))))

(event `Destroy Self`
  ;[1 1 1] Check if the Enemy still has Health left
  (if (<= (`self.EnemyLife`) 0)
    (`self.K2_DestroyActor`)))

(event `self.ReceiveTick`
  (params (DeltaSeconds :type "Float (single-precision)"))
  (bind _spline (`/Game/Blueprints/Enemy/Path.Spline` (`self.Spline REF`)))
  (`self.Decide If Armored or Element Immune`)
  ;[1 1 1] Check if it's burning
  (if (`self.IsBurning`)
    (`self.Burn`))
  ;[1 1 1] If it's slowed due to the ice shot from the turret
  (if (`self.IsSlowed`)
    ;[1 1 1] Move Enemy along spline
    (`TimelineComponent.SetPlayRate` (`self.MoveObject T`) (/ 1.0 (`self.TimeToComplete`)) :!label _label)
    (bind (_direction _movetrack) (`Timeline|MoveObject T`)
      (:`Update`
        (bind _returnvalue (`KismetMathLibrary.Lerp` 0.0 (`SplineComponent.GetSplineLength` (`/Game/Blueprints/Enemy/Path.Spline` (`self.Spline REF`))) _movetrack))
        (`self.K2_SetActorTransform` (`KismetMathLibrary.MakeTransform` (`SplineComponent.GetLocationAtDistanceAlongSpline` _spline _returnvalue "World") (`KismetMathLibrary.RInterpTo_Constant` (`self.K2_GetActorRotation`) (`KismetMathLibrary.Conv_VectorToRotator` (`KismetMathLibrary.GreaterGreater_VectorRotator` (0.0 90.0 0.0) (`SplineComponent.GetRotationAtDistanceAlongSpline` _spline _returnvalue "Local"))) 1.0 5.0)))
        (`self.Destroy Self`)))
    (else
      (`self.Destroy Self`))))

(event `self.ReceiveBeginPlay`
  ;[1 1 1] Get the path for the Enemy to follow
  (bind _returnvalue (`GameplayStatics.GetActorOfClass` "/Game/Blueprints/Enemy/Path.Path_C"))
  (set `self.Spline REF` _returnvalue)
  (`self.Move Object`))

(event `Move Object`
  ;[1 1 1] Move Enemy along spline
  (goto _label))

(event `Decide If Armored or Element Immune`
  (bind _elementalimmune (`self.ElementalImmune`))
  ;[1 1 1] Check Enemy Type
  (if (`self.IsArmored`)
    (if _elementalimmune
      _)
    (elif _elementalimmune
      _)))

(fn `UserConstructionScript`)