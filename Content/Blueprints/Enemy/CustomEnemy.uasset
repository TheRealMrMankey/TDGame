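; CustomEnemy is an enemy actor that follows a spline path and destroys itself about eight seconds after it starts ticking.
; On BeginPlay it randomly picks one of the first two Path actors found.
; A timeline scaled by TimeToComplete moves it along that spline, easing rotation toward a direction perpendicular to the spline's heading.
; Bullets overlapping its box are destroyed, while the enemy itself is unaffected.
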(event `self.ReceiveTick`
  (params (DeltaSeconds :type "Float (single-precision)"))
  (`KismetSystemLibrary.Delay` 8.0)
  (`self.K2_DestroyActor`))

(event `self.ReceiveBeginPlay`
  (bind _outactors (`GameplayStatics.GetAllActorsOfClass` "/Game/Blueprints/Enemy/Path.Path_C"))
  (set `self.Spline REF` (`|GetArrayItem` _outactors (`KismetMathLibrary.RandomInteger` 2)))
  (`self.Move Object`))

(event `Move Object`
  (bind _spline (`/Game/Blueprints/Enemy/Path.Spline` (`self.Spline REF`)))
  (`TimelineComponent.SetPlayRate` (`self.MoveObject T`) (/ 1.0 (`self.TimeToComplete`)))
  (bind (_direction _movetrack) (`Timeline|MoveObject T`)
    (:`Update`
      (set `self.TimeInSpline` _movetrack)
      (bind _returnvalue (`KismetMathLibrary.Lerp` 0.0 (`SplineComponent.GetSplineLength` (`/Game/Blueprints/Enemy/Path.Spline` (`self.Spline REF`))) _movetrack))
      (`self.K2_SetActorTransform` (`KismetMathLibrary.MakeTransform` (`SplineComponent.GetLocationAtDistanceAlongSpline` _spline _returnvalue "World") (`KismetMathLibrary.RInterpTo_Constant` (`self.K2_GetActorRotation`) (`KismetMathLibrary.Conv_VectorToRotator` (`KismetMathLibrary.GreaterGreater_VectorRotator` (0.0 90.0 0.0) (`SplineComponent.GetRotationAtDistanceAlongSpline` _spline _returnvalue "Local"))) 1.0 5.0) (`SceneComponent.K2_GetComponentScale` (`self.EnemyBody`)))))))

(event `self.Box.OnComponentBeginOverlap`
  (params (OverlappedComponent :type "PrimitiveComponent Object Reference") (OtherActor :type "Actor Object Reference") (OtherComp :type "PrimitiveComponent Object Reference") (OtherBodyIndex :type Integer) (bFromSweep :type Boolean) (SweepResult :type "HitResult Structure (by ref)"))
  (bind _asbullet (cast `/Game/Blueprints/Player/Bullet` OtherActor))
  (`self.K2_DestroyActor` _asbullet))

(fn `UserConstructionScript`)