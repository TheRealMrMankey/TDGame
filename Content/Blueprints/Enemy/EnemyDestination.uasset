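; EnemyDestination is the goal point that enemies reach, costing the player health.
; When an EnemyPawn overlaps it, the pawn is destroyed and DamageTaken is subtracted from PlayerHP on the GameManager.
; It then writes the new value straight into the player UI's HP text and plays a LoseLife sound attached to its Audio component.
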(event `self.ReceiveActorBeginOverlap`
  (params (OtherActor :type "Actor Object Reference"))
  (bind _asenemy_pawn (cast `/Game/Blueprints/Enemy/EnemyPawn` OtherActor))
  (`self.K2_DestroyActor` _asenemy_pawn)
  ;[1 1 1] Update Player HP
  (bind _returnvalue (`GameplayStatics.GetActorOfClass` "/Game/Blueprints/Game/GameManager.GameManager_C"))
  (bind _output_get (set `/Game/Blueprints/Game/GameManager.PlayerHP` (- (`/Game/Blueprints/Game/GameManager.PlayerHP` _returnvalue) (`self.DamageTaken`)) _returnvalue))
  (set `TextBlock.Text` (`KismetTextLibrary.Conv_StringToText` (`KismetStringLibrary.Conv_IntToString` _output_get)) (`/Game/Blueprints/UI/PlayerUI.PlayerHP_Text` (`/Game/Blueprints/Game/GameManager.PlayerUI_Var` _returnvalue)))
  (`GameplayStatics.SpawnSoundAttached` "/Game/Audio/LoseLife.LoseLife" (`self.Audio`) "None" (0.0 0.0 0.0) (struct) "KeepRelativeOffset" false 1.0 1.0 0.0 null null))

(fn `UserConstructionScript`)